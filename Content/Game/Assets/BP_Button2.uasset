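; BP_Button2 is an interactable button that adds to a shared button score and records its state in BP_GameInstance.
; Interact alternates through a FlipFlop: one press drops the root 1000 units, increments ButtonScore and sets Button2State, the next only restores the position.
; BeginPlay reapplies the lowered position when Button2State is already set, without advancing the FlipFlop.
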(event EventBeginPlay
  (bind _asbp_game_instance (Utilities|Casting|CastToBP_GameInstance (Game|GetGameInstance)))
  (bind _output_get (Variables|Default|SetAs%20BP%20Game%20Instance _asbp_game_instance))
  (if (Variables|/Game/Game/BP_GameInstance.BP_GameInstance_C|GetButton2State _output_get)
    (Transformation|SetRelativeLocation (Variables|Default|GetDefaultSceneRoot) "0.000000,0.000000,-1000.000000" false false)))

(event Collision|EventActorBeginOverlap
  (params (OtherActor :type Actor%20Object%20Reference)))

(event EventTick
  (params (DeltaSeconds :type Float%20%28single-precision%29)))

(event EventInteract
  (bind _defaultsceneroot (Variables|Default|GetDefaultSceneRoot))
  (bind _as_bp_game_instance (Variables|Default|GetAs%20BP%20Game%20Instance))
  (Utilities|FlowControl|FlipFlop
    (:A
      (Transformation|SetRelativeLocation _defaultsceneroot "0.000000,0.000000,-1000.000000" false false)
      (Variables|/Game/Game/BP_GameInstance.BP_GameInstance_C|SetButtonScore _as_bp_game_instance (+ 1 (Variables|/Game/Game/BP_GameInstance.BP_GameInstance_C|GetButtonScore _as_bp_game_instance)))
      (Variables|/Game/Game/BP_GameInstance.BP_GameInstance_C|SetButton2State _as_bp_game_instance true))
    (:B
      (Transformation|SetRelativeLocation _defaultsceneroot "0, 0, 0" false false))))

(fn ConstructionScript)