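; A key-locked green door that opens by dropping its Cube far below its relative origin.
; Interact alternates through a FlipFlop between opening, only when the GameInstance's GreenKeyScore is 1, and returning the Cube to its origin.
; Opening sets GreenDoorState in BP_GameInstance, which BeginPlay reads to restore the open position.
; Closing never clears that flag, and a failed open attempt still advances the FlipFlop.
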(event EventBeginPlay
  (bind _asbp_game_instance (Utilities|Casting|CastToBP_GameInstance (Game|GetGameInstance)))
  (Variables|Default|SetAs%20BP%20Game%20Instance _asbp_game_instance)
  (if (stale EventInteract _output_get)
    (Transformation|SetRelativeLocation (Variables|Default|GetCube) "0.000000,0.000000,-1000.000000" false false)))

(event Collision|EventActorBeginOverlap
  (params (OtherActor :type Actor%20Object%20Reference)))

(event EventTick
  (params (DeltaSeconds :type Float%20%28single-precision%29)))

(event EventInteract
  (bind _as_bp_game_instance (Variables|Default|GetAs%20BP%20Game%20Instance))
  (Utilities|FlowControl|FlipFlop
    (:A
      (if (== (Variables|/Game/Game/BP_GameInstance.BP_GameInstance_C|GetGreenKeyScore _as_bp_game_instance) 1)
        (bind _output_get (Variables|/Game/Game/BP_GameInstance.BP_GameInstance_C|SetGreenDoorState _as_bp_game_instance true))
        (Transformation|SetRelativeLocation (Variables|Default|GetCube) "0.000000,0.000000,-1000.000000" false false)))
    (:B
      (Transformation|SetRelativeLocation (Variables|Default|GetCube) "0, 0, 0" false false))))

(fn ConstructionScript)