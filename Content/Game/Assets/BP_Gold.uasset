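; BP_Gold is a gold pickup actor whose collected state is stored in BP_GameInstance.
; On BeginPlay it caches the game instance and destroys itself if GoldState is already set.
; Any actor overlap sets GoldState to true without destroying the gold, so removal only happens on a later BeginPlay.
; Tick spins the root component by a fixed step each frame, independent of delta time.
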(event EventBeginPlay
  (bind _asbp_game_instance (Utilities|Casting|CastToBP_GameInstance (Game|GetGameInstance)))
  (bind _output_get (Variables|Default|SetAs%20BP%20Game%20Instance _asbp_game_instance))
  (if (Variables|/Game/Game/BP_GameInstance.BP_GameInstance_C|GetGoldState _output_get)
    (Actor|DestroyActor)))

(event Collision|EventActorBeginOverlap
  (params (OtherActor :type Actor%20Object%20Reference))
  (Variables|/Game/Game/BP_GameInstance.BP_GameInstance_C|SetGoldState (Variables|Default|GetAs%20BP%20Game%20Instance) true))

(event EventTick
  (params (DeltaSeconds :type Float%20%28single-precision%29))
  (Transformation|AddRelativeRotation (Variables|Default|GetDefaultSceneRoot) "0.000000,3.000000,0.000000" false false))

(fn ConstructionScript)