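; BP_FinalDoor is a door that opens only when the game instance's ButtonScore equals 2.
; It opens by instantly moving its root to Z -1000, either on BeginPlay or on Interact with a key sound.
; Interact alternates through a FlipFlop, with the second branch zeroing the Cube's relative location rather than restoring the moved root.
; The FlipFlop advances even when the score check fails.
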(event EventBeginPlay
  (bind _asbp_game_instance (Utilities|Casting|CastToBP_GameInstance (Game|GetGameInstance)))
  (Variables|Default|SetAs%20BP%20Game%20Instance _asbp_game_instance)
  (if (== (Variables|/Game/Game/BP_GameInstance.BP_GameInstance_C|GetButtonScore (Variables|Default|GetAs%20BP%20Game%20Instance)) 2)
    (Transformation|SetRelativeLocation (Variables|Default|GetDefaultSceneRoot) "0.000000,0.000000,-1000.000000" false false)))

(event Collision|EventActorBeginOverlap
  (params (OtherActor :type Actor%20Object%20Reference)))

(event EventTick
  (params (DeltaSeconds :type Float%20%28single-precision%29)))

(event EventInteract
  (Utilities|FlowControl|FlipFlop
    (:A
      (if (== (Variables|/Game/Game/BP_GameInstance.BP_GameInstance_C|GetButtonScore (Variables|Default|GetAs%20BP%20Game%20Instance)) 2)
        (Audio|PlaySound2D "/Game/Game/SFX/keysound.keysound" 1.0 1.0 0.0 0 0)
        (Transformation|SetRelativeLocation (Variables|Default|GetDefaultSceneRoot) "0.000000,0.000000,-1000.000000" false false)))
    (:B
      (Transformation|SetRelativeLocation (Variables|Default|GetCube) "0, 0, 0" false false))))

(fn ConstructionScript)