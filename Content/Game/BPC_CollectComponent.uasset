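; BPC_CollectComponent is a component that handles picking up collectibles and adding their value to the game's score.
; On BeginPlay it caches the BP_GameInstance and copies its GoldState, which is not used elsewhere in this graph.
; Collect adds the collectible's Value to the Score held on the game instance, then tells the collectible to destroy itself.
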(event EventBeginPlay
  (bind _asbp_game_instance (Utilities|Casting|CastToBP_GameInstance (Game|GetGameInstance)))
  (bind _output_get (Variables|Default|SetBP%20Game%20Instance _asbp_game_instance))
  (Variables|Default|SetGold%20State (Variables|/Game/Game/BP_GameInstance.BP_GameInstance_C|GetGoldState _output_get)))

(event EventTick
  (params (DeltaSeconds :type Float%20%28single-precision%29)))

(fn Collect
  (params (Collectible :type BPC%20Collectible%20Component%20Object%20Reference))
  (bind _bp_game_instance (Variables|Default|GetBP%20Game%20Instance))
  (Variables|/Game/Game/BP_GameInstance.BP_GameInstance_C|SetScore _bp_game_instance (+ (Variables|/Game/Game/BPC_CollectibleComponent.BPC_CollectibleComponent_C|GetValue Collectible) (Variables|/Game/Game/BP_GameInstance.BP_GameInstance_C|GetScore _bp_game_instance)))
  (Default|DestroyBPCollectible Collectible))