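; BP_FutureKey is a spinning pickup that records the blue key as collected in BP_GameInstance.
; Any actor overlap sets BlueKeyScore to 1 and destroys the key, with no check on what overlapped it.
; On BeginPlay it caches the game instance and destroys itself if the key is already recorded.
; Tick applies a fixed local rotation each frame, so spin speed depends on frame rate.
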(event EventBeginPlay
  (bind _asbp_game_instance (Utilities|Casting|CastToBP_GameInstance (Game|GetGameInstance)))
  (bind _output_get (Variables|Default|SetAs%20BP%20Game%20Instance _asbp_game_instance))
  (if (== (Variables|/Game/Game/BP_GameInstance.BP_GameInstance_C|GetBlueKeyScore _output_get) 1.0)
    (Actor|DestroyActor)))

(event Collision|EventActorBeginOverlap
  (params (OtherActor :type Actor%20Object%20Reference))
  (Variables|/Game/Game/BP_GameInstance.BP_GameInstance_C|SetBlueKeyScore (Variables|Default|GetAs%20BP%20Game%20Instance) 1)
  (Actor|DestroyActor))

(event EventTick
  (params (DeltaSeconds :type Float%20%28single-precision%29))
  (Transformation|AddActorLocalRotation "0.000000,3.000000,0.000000" false false))

(fn ConstructionScript)