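; BP_Tree is an interactable oak tree that swaps to a log and remembers that state in BP_GameInstance.
; Interact shifts the oak mesh far upward out of the way, reveals the log mesh and sets TreeState to true.
; BeginPlay hides the log, then, if TreeState is already set, hides the oak, replaces its mesh with a gizmo placeholder and shows the log.
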(event EventBeginPlay
  (Development|SetHiddeninGame (Variables|Default|GetSM_TreeLogOakB) true false)
  (bind _asbp_game_instance (Utilities|Casting|CastToBP_GameInstance (Game|GetGameInstance)))
  (bind _output_get (Variables|Default|SetAs%20BP%20Game%20Instance _asbp_game_instance))
  (if (Variables|/Game/Game/BP_GameInstance.BP_GameInstance_C|GetTreeState _output_get)
    (Development|SetHiddeninGame (Variables|Default|GetSM_OakAdultBDense) true false)
    (Components|StaticMesh|SetStaticMesh (Variables|Default|GetSM_OakAdultBDense) "/Engine/VREditor/TransformGizmo/TransformGizmoFreeRotation.TransformGizmoFreeRotation")
    (Development|SetHiddeninGame (Variables|Default|GetSM_TreeLogOakB) false false)
    (Variables|/Game/Game/BP_GameInstance.BP_GameInstance_C|SetTreeState (Variables|Default|GetAs%20BP%20Game%20Instance) true)))

(event Collision|EventActorBeginOverlap
  (params (OtherActor :type Actor%20Object%20Reference)))

(event EventTick
  (params (DeltaSeconds :type Float%20%28single-precision%29)))

(event EventInteract
  (Transformation|AddWorldOffset (Variables|Default|GetSM_OakAdultBDense) "0.000000,0.000000,50000.000000" false false)
  (Development|SetHiddeninGame (Variables|Default|GetSM_TreeLogOakB) false false)
  (Variables|/Game/Game/BP_GameInstance.BP_GameInstance_C|SetTreeState (Variables|Default|GetAs%20BP%20Game%20Instance) true))

(fn ConstructionScript)